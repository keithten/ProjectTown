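; BP_House is a themed house preset built on Apparance procedural generation, inheriting its theme handling from a parent class.
; The construction script calls SyncTheme, and GetTheme reads the current theme from integer parameter 1 of the actor's Apparance parameters.
; A theme change rebuilds the Apparance node with the new value, while SetThemeInternal rebuilds only for a nonzero theme.
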(event Collision|EventActorBeginOverlap
  (params (OtherActor :type Actor%20Object%20Reference)))

(event EventTick
  (params (DeltaSeconds :type Float%20%28single-precision%29)))

(event EventBeginPlay
  (|CallParentFunction))

(fn ConstructionScript
  (CallFunction|SyncTheme))

(fn SetThemeInternal
  (params (Theme :type Integer))
  (if (!= 0 Theme) ; Do anything?
    (|ApparanceRebuildNode Theme)))

(fn OnThemeChange
  (|CallParentFunction)
  (|ApparanceRebuildNode (Variables|Default|GetTheme)))

(fn GetTheme
  (bind _returnvalue (Class|ApparanceBlueprintLibrary|GetCurrentParameters self))
  (bind _returnvalue_2 (Class|ApparanceBlueprintLibrary|GetIntegerParameter _returnvalue 1)) ; Get current Theme value
  (return _returnvalue_2))