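; BP_Town is a town preset actor that rebuilds its Apparance procedural content according to a theme.
; The construction script syncs the theme, and a theme change runs the parent handler before triggering a rebuild with the Theme value.
; Set Theme Internal rebuilds only for a non-zero theme, while BeginPlay just defers to the parent.
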(event Collision|EventActorBeginOverlap
  (params (OtherActor :type Actor%20Object%20Reference)))

(event EventTick
  (params (DeltaSeconds :type Float%20%28single-precision%29)))

(event EventBeginPlay
  (|CallParentFunction))

(fn ConstructionScript
  (CallFunction|SyncTheme))

(fn SetThemeInternal
  (params (Theme :type Integer))
  (if (!= 0 Theme) ; Do anything?
    (|ApparanceRebuildNode Theme)))

(fn OnThemeChange
  (|CallParentFunction)
  (|ApparanceRebuildNode (Variables|Default|GetTheme)))