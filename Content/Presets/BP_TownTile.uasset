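; BP_TownTile is a town tile that drives Apparance procedural generation from its world position and a Theme value.
; The construction script converts the actor location to scaled, axis-swapped Apparance space, then rebuilds with a 100-unit grid-snapped bounds frame, world origin and Theme.
; The SetTheme event reads the current theme from the generation parameters and rebuilds only when the requested theme differs.
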(event EventBeginPlay)

(event Collision|EventActorBeginOverlap
  (params (OtherActor :type Actor%20Object%20Reference)))

(event EventTick
  (params (DeltaSeconds :type Float%20%28single-precision%29)))

(event EventSetTheme
  (params (Theme :type Integer))
  (CallFunction|SetThemeInternal Theme))

(fn ConstructionScript
  (bind _returnvalue (Transformation|GetActorLocation))
  (bind (_x _y _z) (Math|Vector|BreakVector _returnvalue))
  (bind _returnvalue_2 (- 0.0 _x))
  (bind _returnvalue_3 (Math|Vector|MakeVector _y _returnvalue_2 _z))
  (bind _returnvalue_4 (* _returnvalue_3 "0.010000,0.010000,0.010000"))
  (bind _returnvalue_5 (+ _returnvalue_4 "50.000000,50.000000,0.000000"))
  (bind _returnvalue_6 (Class|KismetMathLibrary|VectorSnappedtoGrid _returnvalue_5 1e+02))
  (bind _returnvalue_7 (- _returnvalue_6 "50.000000,50.000000,0.000000"))
  (bind _returnvalue_8 (- _returnvalue_7 _returnvalue_4))
  (bind _out (Utilities|FlipY _returnvalue_8))
  (|ApparanceRebuildNode (Class|ApparanceBlueprintLibrary|MakeFramefromBox (Math|Box|MakeBox _out (+ _out "100.000000,100.000000,1.000000"))) (Utilities|FlipY _returnvalue_4) (Variables|Default|GetTheme)))

(fn SetThemeInternal
  (params (Theme :type Integer))
  (bind _theme (CallFunction|GetTheme))
  (if (!= _theme Theme) ; Do anything?
    (|ApparanceRebuildNode Theme)
    (Variables|Default|SetTheme Theme)))

(fn GetTheme
  (bind _returnvalue (Class|ApparanceBlueprintLibrary|GetCurrentParameters self))
  (bind _returnvalue_2 (Class|ApparanceBlueprintLibrary|GetIntegerParameter _returnvalue 5)) ; Get current Theme value
  (return _returnvalue_2))