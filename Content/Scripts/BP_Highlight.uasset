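; Procedural highlight actor that marks the targeted smart object in the town game, styled for the active tool.
; When the target changes, SetHighlight snaps to its transform and rebuilds Apparance geometry from the object's size, the tool's highlight type and the game mode's theme.
; It stays hidden until GenerationComplete fires, and hides when the target is invalid or not a smart object.
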(event EventBeginPlay)

(event Collision|EventActorBeginOverlap
  (params (OtherActor :type Actor%20Object%20Reference)))

(event EventTick
  (params (DeltaSeconds :type Float%20%28single-precision%29)))

(event EventGenerationComplete
  (if (Variables|Internals|GetShow%20When%20Built)
    (Variables|Internals|SetShow%20When%20Built false)
    (Rendering|SetVisibility (Variables|Transformation|GetRootComponent) true true) ; Show
  ))

(fn ConstructionScript)

(fn SetHighlight
  (params (Actor%20To%20Highlight :type Actor%20Object%20Reference) (Active%20Tool :type BI%20Tool%20Interface))
  ;[0 0 0] Changed?
  (if (!= Actor%20To%20Highlight (Variables|Internals|GetHighlighted%20Object))
    (Utilities|IsValid Actor%20To%20Highlight ; On/Off
      (:Is%20Valid
        (bind _asbi_smart_object (Utilities|Casting|CastToBI_SmartObject Actor%20To%20Highlight) ; Is suitable target?
          (:then
            ;[0 0 0] Set up highlight around target
            (Utilities|FlowControl|Sequence
              (:then_0
                (bind _asapparance_entity (Utilities|Casting|CastToApparanceEntity Actor%20To%20Highlight))
                (Variables|Internals|SetHighlighted%20Object _asapparance_entity)
                (Transformation|SetActorTransform (Transformation|GetActorTransform Actor%20To%20Highlight) false true))
              (:then_1
                (bind _size (Default|GetSize _asbi_smart_object))
                (bind _highlight_type (CallFunction|ToolHighlightType Active%20Tool))
                (bind _asbp_town_game_mode (Utilities|Casting|CastToBP_TownGameMode (Game|GetGameMode))
                  (:then
                    (|ApparanceRebuildNode (Class|ApparanceBlueprintLibrary|MakeFramefromBox (Math|Box|MakeBox (Math|Vector|MakeVector 0.0 0.0 (Variables|HighlightProperties|GetHighlight%20Elevation)) (Math|Vector|MakeVector (.X (Math|Vector2D|BreakVector2D _size)) (.Y (Math|Vector2D|BreakVector2D _size)) 0.0))) _highlight_type (Variables|/Game/Scripts/BP_TownGameMode.BP_TownGameMode_C|GetTheme _asbp_town_game_mode)))
                  (:CastFailed
                    _))
                (Rendering|SetVisibility (Variables|Transformation|GetRootComponent) false true) ; Hide until rebuilt
                (Variables|Internals|SetShow%20When%20Built true))))
          (:CastFailed
            ;[0 0 0] Nothing to highlight
            (Rendering|SetVisibility (Variables|Transformation|GetRootComponent) false true :!label _label)
            (Variables|Internals|SetHighlighted%20Object 0)
            (Variables|Internals|SetShow%20When%20Built false))))
      (:Is%20Not%20Valid
        (goto _label)))))

(fn ToolHighlightType
  (params (Tool :type BI%20Tool%20Interface))
  (Utilities|IsValid (Utilities|ToObject(Interface) Tool)
    (:Is%20Valid
      (bind _highlight_type (Default|GetHighlightType Tool))
      (return _highlight_type))
    (:Is%20Not%20Valid
      (return 0) ; default
    )))