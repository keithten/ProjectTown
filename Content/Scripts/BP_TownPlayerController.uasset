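; Town player controller that handles mouse-driven tool use and selection, highlighting and interactive editing of Apparance smart objects.
; Each tick it picks tray tools by deprojecting HUD coordinates through a scene capture, traces entities under the cursor and intersects the mouse ray with the ground plane.
; Left clicks fire instant tools, toggle modal ones, apply them to ground or object targets, or select and drag-edit entities; right click clears the tool.
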(event EventBeginPlay
  (Utilities|FlowControl|Sequence
    (:then_0
      ;[0 0 0] Gather Systems
      (bind _returnvalue (Actor|GetActorOfClass "/Game/Scripts/BP_ToolTray.BP_ToolTray_C"))
      (Variables|Systems|SetTool%20Tray _returnvalue))
    (:then_1
      (bind _returnvalue_2 (Actor|GetActorOfClass "/Script/Engine.SceneCapture2D"))
      (Variables|Systems|SetTool%20Tray%20Camera _returnvalue_2))
    (:then_2
      (bind _returnvalue_3 (Actor|GetActorOfClass "/Game/Scripts/BP_TownCamera.BP_TownCamera_C"))
      (bind _output_get (Variables|Systems|SetMain%20Camera _returnvalue_3))
      (Variables|Systems|SetMain%20HUD (Variables|/Game/Scripts/BP_TownCamera.BP_TownCamera_C|GetHUD _output_get)))
    (:then_3
      ;[0 0 0] Other Setup
      (Editing|InitHighlight))))

(event EventTick
  (params (DeltaSeconds :type Float%20%28single-precision%29))
  (bind (_worldlocation _worlddirection _returnvalue) (Game|Player|ConvertMouseLocationToWorldSpace))
  (bind _worlddirection_2 (Game|Player|ConvertMouseLocationToWorldSpace))
  (bind _returnvalue_2 (* _worlddirection "100000.000000,100000.000000,100000.000000"))
  (bind _returnvalue_3 (+ _worldlocation _returnvalue_2))
  (bind (_t _intersection _returnvalue_4) (Class|KismetMathLibrary|LinePlaneIntersectionOriginNormal _worldlocation _returnvalue_3 "0, 0, 0" "0.000000,0.000000,1.000000"))
  (Utilities|FlowControl|Sequence
    (:then_0
      ;[0 0 0] Tool tray Hit Testing
      (if (not (Variables|Editing|GetCurrently%20Interacting)) ; Interacting, don't track UI
        (bind _uv (Default|GetToolTrayCoordinate (Variables|Systems|GetMain%20HUD))) ; Where on tray is cursor pointing?
        (bind (_outhit _returnvalue_5) (Collision|LineTraceByChannel (.WorldPosition (Class|GameplayStatics|DeprojectSceneCapturetoWorld (Variables|Systems|GetTool%20Tray%20Camera) _uv)) (+ (.WorldPosition (Class|GameplayStatics|DeprojectSceneCapturetoWorld (Variables|Systems|GetTool%20Tray%20Camera) _uv)) (* (.WorldDirection (Class|GameplayStatics|DeprojectSceneCapturetoWorld (Variables|Systems|GetTool%20Tray%20Camera) _uv)) "10000.000000,10000.000000,10000.000000")) "TraceTypeQuery1" true 0 "None"))
        (if _returnvalue_5 ; Hit any objects?
          (bind _asbi_tool (Utilities|Casting|CastToBI_Tool (.HitActor (Collision|BreakHitResult _outhit))) ; Are they tools?
            (:then
              (ToolUI|SetHilightedTool _asbi_tool) ; Tool
            )
            (:CastFailed
              (ToolUI|SetHilightedTool :!label _label) ; No tool
            ))
          (else
            (goto _label)))))
    (:then_1
      ;[0 0 0] Smart Object Hit Testing
      (if (Utilities|Operators|NotEqual(!=) (Variables|Editing|GetCurrent%20Cursor%20Direction) _worlddirection_2 0.0001) ; Cursor Moved
        (Utilities|FlowControl|Sequence
          (:then_0
            (bind _asapparance_entity (Utilities|Casting|CastToApparanceEntity (.HitActor (Collision|BreakHitResult (.HitResult (Game|Player|GetHitResultUnderCursorbyChannel "TraceTypeQuery1" true)))))
              (:then
                (if (not (Variables|ToolUI|GetIs%20Tool%20Under%20Cursor)) ; already hit a tool
                  (bind _output_get (Variables|Editing|SetEntity%20Under%20Cursor _asapparance_entity))
                  (Variables|Editing|SetIs%20Entity%20Under%20Cursor true)
                  (Editing|SetHighlight _output_get)
                  (else
                    (Variables|Editing|SetEntity%20Under%20Cursor 0 :!label _label_2)
                    (Variables|Editing|SetIs%20Entity%20Under%20Cursor false)
                    (Editing|SetHighlight))))
              (:CastFailed
                (goto _label_2))))
          (:then_1
            (bind _output_get_2 (Variables|Editing|SetCurrent%20Cursor%20Direction _worlddirection_2))
            (bind _returnvalue_6 (Class|ApparanceBlueprintLibrary|UpdateInteractiveEditing _output_get_2 (Variables|Editing|GetInteraction%20Button%20State)))
            (if (Math|Boolean|ANDBoolean _returnvalue_6 (not (Variables|Editing|GetCurrently%20Interacting)) (not (Variables|ToolUI|GetIs%20Tool%20Under%20Cursor))) ; Drag started?
              (Variables|Editing|SetCurrently%20Interacting true))))))
    (:then_2
      ;[0 0 0] Ground Target Tracking
      (bind _output_get_3 (Variables|Editing|SetIs%20Valid%20Ground%20Position (and _returnvalue _returnvalue_4)))
      (if _output_get_3
        (Variables|Editing|SetCurrent%20Ground%20Position _intersection)))))

(event Input|MouseEvents|LeftMouseButton
  (params (Key :type Key%20Structure :default "None"))
  (bind _is_tool_active (Variables|ToolUI|GetIs%20Tool%20Active))
  (bind _active_tool (Variables|ToolUI|GetActive%20Tool))
  (bind _active_tool_2 (Variables|ToolUI|GetActive%20Tool))
  (bind _current_cursor_direction (Variables|Editing|GetCurrent%20Cursor%20Direction))
  (bind _entity_under_cursor (Variables|Editing|GetEntity%20Under%20Cursor))
  ;[0 0 0] Button Interaction
  (:Pressed
    (if (and (Variables|ToolUI|GetIs%20Tool%20Under%20Cursor) (not (Variables|Editing|GetCurrently%20Interacting)))
      (bind _flash_tool (ToolUI|ToolButtonInteraction true)) ; TOOL PRESS
      ;[0 0 0] Flash Tool Button?
      (if _flash_tool
        (Utilities|IsValid (Utilities|ToObject(Interface) _active_tool_2)
          (:Is%20Valid
            (Default|Highlight _active_tool_2 false)
            (Default|Select _active_tool_2 true)
            (Utilities|FlowControl|Delay 0.5)
            (Default|Select _active_tool_2 false))))
      (elif _is_tool_active
        (bind _ground_ (ToolUI|GroundToolActive))
        (if _ground_
          (if (Variables|Editing|GetIs%20Valid%20Ground%20Position) ; TOOL USE
            (Default|Activate _active_tool (Variables|Editing|GetCurrent%20Ground%20Position)))
          (else
            (bind _object_ (ToolUI|ObjectToolActive))
            (if _object_
              (bind _asbi_smart_object (Utilities|Casting|CastToBI_SmartObject (Variables|Editing|GetEntity%20Under%20Cursor)))
              (Default|Activate _active_tool "0, 0, 0" _asbi_smart_object))))
        (else
          (Utilities|FlowControl|Sequence
            (:then_0
              (bind _output_get (Variables|Editing|SetInteraction%20Button%20State true))
              (Class|ApparanceBlueprintLibrary|UpdateInteractiveEditing _current_cursor_direction _output_get))
            (:then_1
              ;[0 0 0] Entity Select / Deselect
              (if (Variables|Editing|GetIs%20Entity%20Under%20Cursor)
                (Utilities|Casting|CastToBI_SmartObject _entity_under_cursor ; SO clicked
                  (:then
                    (Variables|Editing|SetClicked%20Entity _entity_under_cursor)
                    (if (Variables|Editing|GetCurrently%20Interacting) ; Used to interact?
                      (Variables|Editing|SetCurrently%20Interacting false) ; Done interacting
                      (else
                        (Utilities|IsValid (Variables|Editing|GetClicked%20Entity) ; Handle as selection click
                          (:Is%20Valid
                            (Editing|EntityClicked (Variables|Editing|GetClicked%20Entity)) ; Select
                            (Default|SetHighlight (Variables|Editing|GetHighlight%20Entity)) ; Un-highlight
                          )))))
                  (:CastFailed
                    (Variables|Editing|SetClicked%20Entity 0 :!label _label) ; Clicked something else
                  ))
                (else
                  (goto _label)))))))))
  (:Released
    (if (and (Variables|ToolUI|GetIs%20Tool%20Under%20Cursor) (not (Variables|Editing|GetCurrently%20Interacting)))
      (ToolUI|ToolButtonInteraction false) ; TOOL RELEASE
      (elif (not _is_tool_active)
        (Utilities|FlowControl|Sequence
          (:then_0
            (bind _output_get_2 (Variables|Editing|SetInteraction%20Button%20State false))
            (Class|ApparanceBlueprintLibrary|UpdateInteractiveEditing _current_cursor_direction _output_get_2))
          (:then_1
            (if (Variables|Editing|GetCurrently%20Interacting) ; Was to interacting?
              (Variables|Editing|SetCurrently%20Interacting false)
              (else
                (Variables|Editing|SetCurrently%20Interacting false)
                (Utilities|IsValid (Variables|Editing|GetClicked%20Entity) ; Handle as deselection click
                  (:Is%20Not%20Valid
                    (Editing|EntityClicked) ; Deselect
                  ))))))))))

(event Input|MouseEvents|RightMouseButton
  (params (Key :type Key%20Structure :default "None"))
  ;[0 0 0] Button Interaction
  (:Pressed
    (ToolUI|SetSelectedTool) ; Clear Active Tool
  ))

(fn ConstructionScript)

(fn EntityClicked
  (params (Actor :type Apparance%20Entity%20Object%20Reference))
  (bind _asbi_smart_object (Utilities|Casting|CastToBI_SmartObject Actor)
    (:then
      _)
    (:CastFailed
      _))
  (if (and (Utilities|IsValid Actor) (Utilities|IsValid (Utilities|ToObject(Interface) _asbi_smart_object))) ; Clicked on a smart object?
    (if (not (== (Variables|Editing|GetSelected%20Entity) Actor)) ; Already selected?
      (Editing|SetSelectedEntity (Variables|Editing|GetSelected%20Entity) false) ; Deselect current
      (Editing|SetSelectedEntity Actor true) ; Select new
    )
    (else
      (Editing|SetSelectedEntity (Variables|Editing|GetSelected%20Entity) false) ; Deselect all
    )))

(fn SetSelectedEntity
  (params (Entity :type Apparance%20Entity%20Object%20Reference) (Selected :type Boolean))
  (Utilities|IsValid Entity ; Anything to select?
    (:Is%20Valid
      (bind _returnvalue (Class|ApparanceEntity|GetEditingSelected Entity))
      (if (!= _returnvalue Selected) ; Any action needed?
        (Class|ApparanceEntity|SetEditingSelected Entity Selected)
        (if Selected ; Just Selected?
          (Variables|Editing|SetSelected%20Entity Entity)
          (else
            (Variables|Editing|SetSelected%20Entity 0) ; We have deselected!
          ))))
    (:Is%20Not%20Valid
      (Variables|Editing|SetSelected%20Entity 0) ; We have deselected!
    )))

(fn SetHilightedTool
  (params (Tool :type BI%20Tool%20Interface))
  (bind _returnvalue (Utilities|ToObject(Interface) Tool))
  (bind _returnvalue_2 (Utilities|IsValid _returnvalue))
  ;[0 0 0] Changed?
  (if (!= (Utilities|ToObject(Interface) (Variables|ToolUI|GetTool%20Hovered)) _returnvalue) ; Changed?
    (Utilities|FlowControl|Sequence
      (:then_0
        ;[0 0 0] Un-highlight Old
        (if (Utilities|IsValid (Utilities|ToObject(Interface) (Variables|ToolUI|GetTool%20Hovered)))
          (Default|Highlight (Variables|ToolUI|GetTool%20Hovered) false) ; un hilight old
        ))
      (:then_1
        ;[0 0 0] Highlight New
        (if _returnvalue_2
          (Default|Highlight Tool true) ; hilight new
        )
        ;[0 0 0] Update State
        (Variables|ToolUI|SetTool%20Hovered Tool) ; Store New
        (Variables|ToolUI|SetIs%20Tool%20Under%20Cursor _returnvalue_2)))))

(fn ToolButtonInteraction
  (params (Pressed :type Boolean))
  (if Pressed
    (bind _instant_ (Default|WantInstantAction (Variables|ToolUI|GetTool%20Hovered)))
    (if _instant_
      (Default|Activate (Variables|ToolUI|GetTool%20Hovered) "0, 0, 0") ; Activate immediately, no parameters
      (return true)
      (else
        (ToolUI|SetSelectedTool (Variables|ToolUI|GetTool%20Hovered)) ; Just modal tools for now.\nBut can reselect to deactivate
        (return false)))))

(fn SetSelectedTool
  (params (Tool :type BI%20Tool%20Interface))
  (bind _returnvalue (Utilities|ToObject(Interface) Tool))
  (bind _returnvalue_2 (Utilities|IsValid _returnvalue))
  ;[0 0 0] Changes?
  (LocalVariables|SetOld%20Tool%20Object (Utilities|ToObject(Interface) (Variables|ToolUI|GetActive%20Tool)))
  (if (or (Utilities|IsValid (Utilities|ToObject(Interface) (Variables|ToolUI|GetActive%20Tool))) _returnvalue_2) ; Any tool changes?
    ;[0 0 0] Action Required
    (Utilities|FlowControl|Sequence
      (:then_0
        (if (Utilities|IsValid (Utilities|ToObject(Interface) (Variables|ToolUI|GetActive%20Tool))) ; Had old tool?
          ;[0 0 0] Deactivate Old Tool
          (Default|Select (Variables|ToolUI|GetActive%20Tool) false)
          (Variables|ToolUI|SetActive%20Tool 0)
          (Variables|ToolUI|SetIs%20Tool%20Active false)))
      (:then_1
        (if (and (!= (LocalVariables|GetOld%20Tool%20Object) _returnvalue) _returnvalue_2) ; Changing tool?
          ;[0 0 0] Activate New Tool
          (Default|Select Tool true)
          (Variables|ToolUI|SetActive%20Tool Tool)
          (Variables|ToolUI|SetIs%20Tool%20Active true))))))

(fn InitHighlight
  (bind _returnvalue (Game|SpawnActorfromClass "/Game/Scripts/BP_Highlight.BP_Highlight_C" (Math|Transform|MakeTransform "0, 0, 0") "Undefined" "MultiplyWithRoot" 0 0))
  (Variables|Editing|SetHighlight%20Entity _returnvalue)
  (Editing|SetHighlight) ; Hide initially
)

(fn SetHighlight
  (params (Actor%20To%20Highlight :type Actor%20Object%20Reference))
  (bind _active_tool (Variables|ToolUI|GetActive%20Tool))
  (bind _highlight_entity (Variables|Editing|GetHighlight%20Entity))
  ;[0 0 0] Reject current selection or during interaction/placement
  (bind _object_ (ToolUI|ObjectToolActive))
  (if (Math|Boolean|ORBoolean (== (Variables|Editing|GetSelected%20Entity) Actor%20To%20Highlight) (Variables|Editing|GetCurrently%20Interacting) (and (Variables|ToolUI|GetIs%20Tool%20Active) (not _object_)))
    (Default|SetHighlight _highlight_entity 0 _active_tool) ; No Highlight
    (else
      (Default|SetHighlight _highlight_entity Actor%20To%20Highlight _active_tool) ; Highlight
    )))

(fn GroundToolActive
  (if (Variables|ToolUI|GetIs%20Tool%20Active)
    (bind _hit_ground (Default|WantGroundTarget (Variables|ToolUI|GetActive%20Tool)))
    (return _hit_ground)
    (else
      (return false) ; No tool
    )))

(fn ObjectToolActive
  (if (Variables|ToolUI|GetIs%20Tool%20Active)
    (bind _hit_object (Default|WantObjectTarget (Variables|ToolUI|GetActive%20Tool)))
    (return _hit_object)
    (else
      (return false) ; no tool
    )))