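; BP_Tool is a selectable tool that, by default, places an object by spawning its SpawnClass at a target ground position.
; Highlight and Select set state flags, which ApplyState packs into a bitmask for an Apparance rebuild of its appearance.
; Getter functions supply help text, hover text and highlight type.
; Targeting and instant-action queries all return false here, reading as defaults for specialized tools to override.
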(event EventBeginPlay)

(event Collision|EventActorBeginOverlap
  (params (OtherActor :type Actor%20Object%20Reference)))

(event EventTick
  (params (DeltaSeconds :type Float%20%28single-precision%29)))

(event EventHighlight
  (params (Enable :type Boolean))
  (Variables|Default|SetIs%20Highlighted Enable)
  (CallFunction|ApplyState))

(event EventSelect
  (params (Enable :type Boolean))
  (Variables|Default|SetIs%20Selected Enable)
  (CallFunction|ApplyState))

(event EventActivate
  (params (Target%20Ground%20Pos :type Vector :default "0, 0, 0") (Target%20Object :type BI%20Smart%20Object%20Interface))
  ;[0 0 0] Default Behavoir: Place Object
  (bind _asactor (Utilities|Casting|CastToActorClass (Variables|Default|GetSpawn%20Class)))
  (Game|SpawnActorfromClass _asactor (Math|Transform|MakeTransform Target%20Ground%20Pos) "AlwaysSpawn" "MultiplyWithRoot" 0 0))

(fn ConstructionScript)

(fn ApplyState
  (|ApparanceRebuildNode (Class|KismetMathLibrary|OrIntInt (Math|Integer|SelectInt 1 0 (Variables|Default|GetIs%20Highlighted)) (Math|Integer|SelectInt 2 0 (Variables|Default|GetIs%20Selected)))))

(fn GetHelpText
  (return (Variables|Default|GetTool%20Help%20Text)))

(fn GetHighlightType
  (return 0))

(fn GetHoverText
  (return (Variables|Default|GetButton%20Hover%20Text)))

(fn WantGroundTarget
  (return false))

(fn WantInstantAction
  (return false))

(fn WantObjectTarget
  (return false))