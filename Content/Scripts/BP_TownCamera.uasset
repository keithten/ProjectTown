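; BP_TownCamera is an RTS-style town camera actor that also brings up the HUD when play begins.
; On BeginPlay, outside dedicated servers, it makes its RTSCamera component the active camera, then creates a UI_HUD widget, stores it and adds it to the viewport.
; Tick, overlap and construction script carry no logic of their own.
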(event EventBeginPlay
  (|CallParentFunction)
  (if (not (Networking|IsDedicatedServer))
    (Utilities|FlowControl|Sequence
      (:then_0
        ;[0 0 0] Camera Setup
        (Class|RTSCamera|SetActiveCamera (Variables|Default|GetRTSCamera)))
      (:then_1
        ;[0 0 0] HUD Setup
        (bind _returnvalue (UserInterface|CreateWidget "/Game/Scripts/UI/UI_HUD.UI_HUD_C"))
        (bind _output_get (Variables|Default|SetHUD _returnvalue))
        (UserInterface|Viewport|AddtoViewport _output_get 0)))))

(event Collision|EventActorBeginOverlap
  (params (OtherActor :type Actor%20Object%20Reference))
  (|CallParentFunction OtherActor) ; This node is disabled and will not be called.\nDrag off pins to build functionality.
)

(event EventTick
  (params (DeltaSeconds :type Float%20%28single-precision%29))
  (|CallParentFunction DeltaSeconds) ; This node is disabled and will not be called.\nDrag off pins to build functionality.
)

(fn ConstructionScript
  (|CallParentFunction))